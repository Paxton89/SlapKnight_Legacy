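; BP_CameraPawn is the camera pawn, which also owns the testing HUD widget.
; On BeginPlay it creates a TestingUI widget, adds it to the viewport and keeps a reference to it.
; Custom events relay to that widget: a failed-click flash, a tile's unit stats, and hover info with a tile and stamina.
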(event EventBeginPlay
  (bind _returnvalue (UserInterface|CreateWidget "/Game/BluePrints/Widgets/TestingUI.TestingUI_C"))
  (UserInterface|Viewport|AddtoViewport _returnvalue 0)
  (Variables|Default|SetwidgetTroll _returnvalue))

(event Collision|EventActorBeginOverlap
  (params (OtherActor :type Actor%20Object%20Reference)))

(event EventTick
  (params (DeltaSeconds :type Float%20%28single-precision%29)))

(event EventHoveringUnitInfo
  (params (tile :type Base%20Tile%20Object%20Reference) (stamina :type Integer))
  (Default|HoverStats (Variables|Default|GetwidgetTroll) tile (Math|Conversions|ToFloat(Integer) stamina)))

(event EventClickFailUI
  (Default|FlashTroll (Variables|Default|GetwidgetTroll)))

(event EventShowUnitStatsUI
  (params (tile :type Base%20Tile%20Object%20Reference))
  (Default|ShowStats (Variables|Default|GetwidgetTroll) tile))

(fn ConstructionScript)